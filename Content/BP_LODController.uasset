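; BP_LODController is an actor that randomly switches the forced LOD of the BP_Gavin character at runtime.
; On BeginPlay it finds a BP_Gavin in the level and caches its LODSync component.
; A self-rescheduling delay loop waits a random interval within configurable bounds, then sets ForcedLOD to a random index up to MaxLODIndex and prints it.
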(event Custom|ScheduleNextLODChange
  (Utilities|FlowControl|Delay (Math|Random|RandomFloatinRange (Variables|Default|GetChangeIntervalMin) (Variables|Default|GetChangeIntervalMax)))
  (CallFunction|ChangeLOD)
  (CallFunction|ScheduleNextLODChange))

(event Custom|ChangeLOD
  (bind _output_get (Variables|Default|SetLODIndex (Math|Random|RandomIntegerinRange 0 (Variables|Default|GetMaxLODIndex))))
  (Variables|/Script/Engine.LODSyncComponent|SetForcedLOD (Variables|Default|GetLODSyncComp) _output_get)
  (Development|PrintString (Utilities|String|ToString(Integer) _output_get)))

(event EventBeginPlay
  (Development|PrintString "BP_LODController started")
  (bind _returnvalue (Actor|GetActorOfClass "/Game/MetaHumans/Gavin/BP_Gavin.BP_Gavin_C"))
  (Utilities|IsValid (Variables|/Game/MetaHumans/Gavin/BP_Gavin.BP_Gavin_C|GetLODSync _returnvalue)
    (:Is%20Valid
      (Variables|Default|SetLODSyncComp (Variables|/Game/MetaHumans/Gavin/BP_Gavin.BP_Gavin_C|GetLODSync _returnvalue))
      (CallFunction|ScheduleNextLODChange))
    (:Is%20Not%20Valid
      (Development|PrintString "Invalid"))))

(event Collision|EventActorBeginOverlap
  (params (OtherActor :type Actor%20Object%20Reference)))

(event EventTick
  (params (DeltaSeconds :type Float%20%28single-precision%29)))

(fn ConstructionScript)